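; AI controller for guard NPCs that runs the Guard_Behavior tree on the PatrolData blackboard.
; Perception updates for actors without the "Enemy" tag set EnemyKey when sensed and clear it when lost.
; Each tick it sets the possessed PatrollingGuard2's Aiming and Shooting flags to whether the controller has a valid focus actor.
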(event OnTargetPerceptionUpdated(AIPerception)
  (params (Actor :type Actor%20Object%20Reference) (Stimulus :type AI%20Stimulus%20Structure))
  (bind _enemy_key (Variables|Default|GetEnemy%20Key))
  (bind _blackboardcomp (Variables|Default|GetBlackboardComp))
  (if (not (Actor|ActorHasTag Actor "Enemy"))
    (if (.bSuccessfullySensed (Utilities|Struct|BreakAIStimulus Stimulus))
      (AI|Components|Blackboard|SetValueasObject _blackboardcomp _enemy_key Actor)
      (else
        (AI|Components|Blackboard|ClearValue _blackboardcomp _enemy_key)))))

(event EventBeginPlay
  (bind _blackboardcomponent (Class|AIController|UseBlackboard "/Game/Dynamic/NPC/AI/PatrolData.PatrolData"))
  (AI|RunBehaviorTree "/Game/Dynamic/NPC/AI/Guard_Behavior.Guard_Behavior")
  (Variables|Default|SetBlackboardComp _blackboardcomponent))

(event EventTick
  (params (DeltaSeconds :type Float%20%28single-precision%29))
  (bind _aspatrolling_guard_2 (Utilities|Casting|CastToPatrollingGuard2 (Pawn|GetControlledPawn)))
  (bind _output_get (Variables|/Game/Dynamic/NPC/Behavior/PatrollingGuard2.PatrollingGuard2_C|SetAiming _aspatrolling_guard_2 (Utilities|IsValid (Class|AIController|GetFocusActor))))
  (Variables|/Game/Dynamic/NPC/Behavior/PatrollingGuard2.PatrollingGuard2_C|SetShooting _aspatrolling_guard_2 _output_get))

(fn ConstructionScript)