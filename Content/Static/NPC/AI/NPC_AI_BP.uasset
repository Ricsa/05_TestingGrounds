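; AI controller for guard NPCs that tracks perceived actors as targets.
; On BeginPlay it initializes the PatrolData blackboard and runs the Guard_Behavior behavior tree.
; AI perception updates write any sensed actor without the "Enemy" tag to the blackboard's enemy key, and clear that key when such an actor is lost.
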(event OnTargetPerceptionUpdated(AIPerception)
  (params (Actor :type Actor%20Object%20Reference) (Stimulus :type AI%20Stimulus%20Structure))
  (bind _enemy_key (Variables|Default|GetEnemy%20Key))
  (bind _blackboardcomp (Variables|Default|GetBlackboardComp))
  (if (not (Actor|ActorHasTag Actor "Enemy"))
    (if (.bSuccessfullySensed (Utilities|Struct|BreakAIStimulus Stimulus))
      (AI|Components|Blackboard|SetValueasObject _blackboardcomp _enemy_key Actor)
      (else
        (AI|Components|Blackboard|ClearValue _blackboardcomp _enemy_key)))))

(event EventBeginPlay
  (bind _blackboardcomponent (Class|AIController|UseBlackboard "/Game/Static/NPC/AI/PatrolData.PatrolData"))
  (AI|RunBehaviorTree "/Game/Static/NPC/AI/Guard_Behavior.Guard_Behavior")
  (Variables|Default|SetBlackboardComp _blackboardcomponent))

(fn ConstructionScript)